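; BP_Explosion is a short-lived explosion actor that kills bomber characters it touches.
; On overlap, it casts the other actor to BP_BomberCharacter and destroys it.
; Each tick it accumulates a timer, shrinks its sphere collision's world scale linearly by a shrink speed, and destroys itself once the scale drops below zero.
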(event EventBeginPlay)

(event Collision|EventActorBeginOverlap
  (params (OtherActor :type Actor%20Object%20Reference))
  (Utilities|FlowControl|Sequence
    (:then_0
      (bind _asbp_bomber_character (Utilities|Casting|CastToBP_BomberCharacter OtherActor))
      (Actor|DestroyActor _asbp_bomber_character))))

(event EventTick
  (params (DeltaSeconds :type Float%20%28single-precision%29))
  (bind _output_get (Variables|Default|SetExplosionTimer (+ (Variables|Default|GetExplosionTimer) DeltaSeconds)))
  (Transformation|SetWorldScale3D (Variables|Default|GetSphereCollision) (Math|Vector|MakeVector (- 1.0 (* _output_get (Variables|Default|GetExplosionShrinkSpeed))) (- 1.0 (* _output_get (Variables|Default|GetExplosionShrinkSpeed))) (- 1.0 (* _output_get (Variables|Default|GetExplosionShrinkSpeed)))))
  (if (< (- 1.0 (* _output_get (Variables|Default|GetExplosionShrinkSpeed))) 0.0)
    (Actor|DestroyActor)))

(fn ConstructionScript)