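; Bomberman-style bomb that detonates on a timer with a growing, color-shifting fuse, or skips the timer when remote, and turns solid once a player steps off.
; Explode steps outward in four directions, spawning explosions, destroying blocks and pickups, and flagging blocked directions with negative Z.
; Bombs it hits chain-explode, with IsDead preventing loops.
; OnExploded notifies the instigating character and game mode; chained bombs skip the win check.
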(event Custom|OnBombExploded
  (bind _returnvalue (Game|GetInstigator))
  ;[1 1 1] When any bomb explodes, signal the gamemode to update the hud, and the player's bomb count
  (Utilities|IsValid _returnvalue
    (:Is%20Valid
      (bind _asbp_bomber_character (Utilities|Casting|CastToBP_BomberCharacter _returnvalue))
      (Default|OnBombExploded _asbp_bomber_character)
      (bind _asbp_bomber_game_mode (Utilities|Casting|CastToBP_BomberGameMode (Game|GetGameMode)))
      (Default|OnBombExploded _asbp_bomber_game_mode _asbp_bomber_character))))

(event Custom|TickBombTimer
  (params (DeltaSeconds :type Float%20%28single-precision%29))
  ;[1 1 1] Growing "fuse" effect
  (Variables|Default|SetBombTimer (+ (Variables|Default|GetBombTimer) DeltaSeconds))
  (Utilities|FlowControl|Sequence
    (:then_0
      (Rendering|Material|SetVectorParameterValue (Variables|Default|GetDynamicFuseMaterial) "Color" (Utilities|Struct|MakeLinearColor 1.0 (- 1.0 (/ (Variables|Default|GetBombTimer) 2.0)) 0.0 1.0) :!class /Script/Engine.MaterialInstanceDynamic))
    (:then_1
      (Transformation|SetRelativeScale3D (Variables|Default|GetFuse) (Math|Vector|MakeVector (/ (Variables|Default|GetBombTimer) (Variables|Default|GetBombFuseTime)) (/ (Variables|Default|GetBombTimer) (Variables|Default|GetBombFuseTime)) (/ (Variables|Default|GetBombTimer) (Variables|Default|GetBombFuseTime)))))
    (:then_2
      (if (> (Variables|Default|GetBombTimer) (Variables|Default|GetBombFuseTime))
        (CallFunction|Explode)
        (Actor|Tick|SetActorTickEnabled false)))))

(event Custom|ChainExplosion
  (params (InParentBomb :type BP%20Bomb%20Object%20Reference))
  ;[1 1 1] Fires if this bomb is triggered by another bomb
  (Variables|Default|SetParentBomb InParentBomb)
  (Variables|Default|SetBombTimer (Variables|Default|GetBombFuseTime))
  (CallFunction|Explode)
  (Actor|Tick|SetActorTickEnabled false))

(event Custom|GameMode_CheckGameEnded
  ;[1 1 1] Check the win conditions to see if any player won as a result of this bomb exploding
  (bind _asbp_bomber_game_mode (Utilities|Casting|CastToBP_BomberGameMode (Game|GetGameMode)))
  (Default|CheckGameEnded _asbp_bomber_game_mode))

(event Custom|Explode
  (bind _spherecollision (Variables|Default|GetSphereCollision))
  ;[1 1 1] Blow up this bomb, placing explosions in the 4 cardinal directions
  (Utilities|FlowControl|Sequence
    (:then_0
      (Variables|/Script/Engine.PrimitiveComponent|SetbGenerateOverlapEvents _spherecollision false)
      (Collision|SetCollisionResponsetoAllChannels _spherecollision "ECR_Ignore")
      (Variables|Default|SetIsDead true) ; Mark this bomb as dead, to avoid an infinite loop
      (Game|SpawnActorfromClass "/Game/Actors/BP_Explosion.BP_Explosion_C" (Transformation|GetActorTransform) "Undefined" self (Variables|Default|GetParentBomb) (Variables|Default|GetInstigator))
      (for _index (range 1 (Variables|Default|GetExplosionSize))
        (for (_array_element _array_index) (Variables|Default|GetExplosionTransforms)
          (bind (_outactors _returnvalue) (Collision|SphereOverlapActors (+ (Transformation|GetActorLocation) (* _array_element _index)) 38.0 (Utilities|Array|MakeArray "ObjectTypeQuery1" "ObjectTypeQuery6") 0 (Utilities|Array|MakeArray self))) ; Check each bomb explosion location for actors
          (if _returnvalue
            (bind _array_element_2 (Utilities|Array|ForEachLoopwithBreak _outactors :!label _label)
              (:LoopBody
                ;[1 1 1] If this bomb triggered another bomb, we will not check the win conditions at the end of this function
                (bind _asbp_bomb (Utilities|Casting|CastToBP_Bomb _array_element_2)
                  (:then
                    (if (not (Variables|BP_Bomb_C|GetIsDead _asbp_bomb))
                      (Variables|BP_Bomb_C|SetIsDead _asbp_bomb true)
                      (EventDispatchers|UnbindEventfromOnExploded _asbp_bomb (delegate Custom|GameMode_CheckGameEnded))
                      (Utilities|Array|Add (Variables|Default|GetChainedBombs) _asbp_bomb)
                      (goto _label Break)))
                  (:CastFailed
                    ;[1 1 1] If we found a destructible block, destroy it
                    (bind _asbp_destructible_block (Utilities|Casting|CastToBP_DestructibleBlock _array_element_2)
                      (:then
                        (Actor|DestroyActor _asbp_destructible_block)
                        (Game|SpawnActorfromClass "/Game/Actors/BP_Explosion.BP_Explosion_C" (Math|Transform|MakeTransform (+ (Transformation|GetActorLocation) (* _array_element _index)) "0, 0, 0" "1,1,1") "Undefined" self (Variables|Default|GetParentBomb) (Variables|Default|GetInstigator))
                        (goto _label Break))
                      (:CastFailed
                        (bind _asbp_pickup (Utilities|Casting|CastToBP_Pickup _array_element_2))
                        (Actor|DestroyActor _asbp_pickup)
                        (goto _label Break))))))
              (:Completed
                ;[1 1 1] If we found any actors at the location, mark the explosion to stop in that direction
                (|SetBy-RefVar (Utilities|Array|Get(acopy) (Variables|Default|GetExplosionTransforms) _array_index) "0.000000,0,-1.000000")))
            (elif (not (< (.Z (Math|Vector|BreakVector (Utilities|Array|Get(acopy) (Variables|Default|GetExplosionTransforms) _array_index))) 0.0))
              (Game|SpawnActorfromClass "/Game/Actors/BP_Explosion.BP_Explosion_C" (Math|Transform|MakeTransform (+ (Transformation|GetActorLocation) (* _array_element _index)) "0, 0, 0" "1,1,1") "Undefined" self (Variables|Default|GetParentBomb) (Variables|Default|GetInstigator)))))
        ;[1 1 1] After we're done exploding this bomb, blow up any other bombs that this bomb triggered
        (for _array_element_3 (Variables|Default|GetChainedBombs)
          (CallFunction|ChainExplosion _array_element_3 (Variables|Default|GetParentBomb)))
        (Utilities|Array|Clear (Variables|Default|GetChainedBombs))))
    (:then_1
      (Rendering|SetActorHiddenInGame true)
      (Default|CallOnExploded) ; If bound, this dispatcher will check the win conditions
      (Actor|DestroyActor))))

(event EventBeginPlay
  (if (Variables|Default|GetIsActive)
    (if (Variables|Default|GetIsRemote)
      ;[1 1 1] For remote bombs, change their color, and disable the "fuse" effect
      (Actor|Tick|SetActorTickEnabled false)
      (Rendering|Material|SetMaterial (Variables|Default|GetFuse) 0 "/Game/Materials/M_RemoteBombFuse.M_RemoteBombFuse")
      (else
        ;[1 1 1] For regular bombs, have the "fuse" grow and change color over time
        (bind _returnvalue (Rendering|Material|CreateDynamicMaterialInstance (Variables|Default|GetFuse) 0 (Rendering|Material|GetMaterial (Variables|Default|GetFuse) 0) :!class /Script/Engine.PrimitiveComponent))
        (Variables|Default|SetDynamicFuseMaterial _returnvalue)
        (Transformation|SetWorldScale3D (Variables|Default|GetFuse) "0, 0, 0")))
    (Variables|Default|SetParentBomb self)
    (EventDispatchers|BindEventtoOnExploded (delegate Custom|GameMode_CheckGameEnded))
    (EventDispatchers|BindEventtoOnExploded (delegate Custom|OnBombExploded))
    (else
      (Actor|Tick|SetActorTickEnabled false))))

(event Collision|EventActorBeginOverlap
  (params (OtherActor :type Actor%20Object%20Reference)))

(event EventTick
  (params (DeltaSeconds :type Float%20%28single-precision%29))
  (CallFunction|TickBombTimer DeltaSeconds))

(event Collision|EventActorEndOverlap
  (params (OtherActor :type Actor%20Object%20Reference))
  ;[1 1 1] Make solid once the player walks off of the bomb
  (Utilities|Casting|CastToBP_BomberCharacter OtherActor)
  (Collision|SetCollisionResponsetoChannel (Variables|Default|GetSphereCollision) "ECC_Pawn" "ECR_Block"))

(fn ConstructionScript)