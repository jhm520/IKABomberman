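; A pickup actor that increases a bomber character's bomb blast length when collected.
; It overrides the parent pickup's give-to-player event to increment the character's BombExplosionSize by one, then calls the parent implementation.
; All other behavior comes from the parent class; the construction script only calls its parent.
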(event EventBeginPlay
  (|CallParentFunction))

(event Collision|EventActorBeginOverlap
  (params (OtherActor :type Actor%20Object%20Reference))
  (|CallParentFunction OtherActor))

(event EventTick
  (params (DeltaSeconds :type Float%20%28single-precision%29))
  (|CallParentFunction DeltaSeconds))

(event EventGivePickuptoPlayer
  (params (InBomberCharacter :type BP%20Bomber%20Character%20Object%20Reference))
  (Utilities|FlowControl|Sequence
    (:then_0
      (Math|Integer|IncrementInt (Variables|/Game/Characters/BP_BomberCharacter.BP_BomberCharacter_C|GetBombExplosionSize InBomberCharacter)))
    (:then_1
      (|CallParentFunction InBomberCharacter))))

(fn ConstructionScript
  (|CallParentFunction))