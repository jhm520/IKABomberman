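; Bomb-capacity pickup for a Bomberman-style game that grants the collecting character one more bomb.
; GivePickuptoPlayer increments both the character's current and maximum bomb counts, then notifies BP_BomberGameMode that the player's bomb count changed.
; A sequence then calls the parent pickup's give logic, which still runs if the game mode cast fails.
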(event EventBeginPlay
  (|CallParentFunction))

(event Collision|EventActorBeginOverlap
  (params (OtherActor :type Actor%20Object%20Reference))
  (|CallParentFunction OtherActor))

(event EventTick
  (params (DeltaSeconds :type Float%20%28single-precision%29))
  (|CallParentFunction DeltaSeconds))

(event EventGivePickuptoPlayer
  (params (InBomberCharacter :type BP%20Bomber%20Character%20Object%20Reference))
  (Utilities|FlowControl|Sequence
    (:then_0
      (Math|Integer|IncrementInt (Variables|/Game/Characters/BP_BomberCharacter.BP_BomberCharacter_C|GetCurrentBombs InBomberCharacter)
        (:%20%20
          (Math|Integer|IncrementInt (Variables|/Game/Characters/BP_BomberCharacter.BP_BomberCharacter_C|GetMaxBombs InBomberCharacter)
            (:%20%20
              (bind _asbp_bomber_game_mode (Utilities|Casting|CastToBP_BomberGameMode (Game|GetGameMode)))
              (Default|OnPlayerBombCountChanged _asbp_bomber_game_mode InBomberCharacter))))))
    (:then_1
      (|CallParentFunction InBomberCharacter))))

(fn ConstructionScript
  (|CallParentFunction))