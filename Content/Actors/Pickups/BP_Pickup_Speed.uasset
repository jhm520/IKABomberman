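; Speed pickup actor that makes the collecting bomber character walk faster.
; On GivePickuptoPlayer it adds a fifth of the character's default walk speed to the current max walk speed, so repeated pickups stack linearly.
; It then hands off to the parent pickup's implementation of the same event; the other events and the construction script add no logic of their own.
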(event EventBeginPlay
  (|CallParentFunction))

(event Collision|EventActorBeginOverlap
  (params (OtherActor :type Actor%20Object%20Reference))
  (|CallParentFunction OtherActor))

(event EventTick
  (params (DeltaSeconds :type Float%20%28single-precision%29))
  (|CallParentFunction DeltaSeconds))

(event EventGivePickuptoPlayer
  (params (InBomberCharacter :type BP%20Bomber%20Character%20Object%20Reference))
  (bind _charactermovement (Variables|/Script/Engine.Character|GetCharacterMovement InBomberCharacter))
  (Utilities|FlowControl|Sequence
    (:then_0
      (Variables|/Script/Engine.CharacterMovementComponent|SetMaxWalkSpeed _charactermovement (+ (Variables|/Script/Engine.CharacterMovementComponent|GetMaxWalkSpeed _charactermovement) (* (Variables|/Game/Characters/BP_BomberCharacter.BP_BomberCharacter_C|GetDefaultWalkSpeed InBomberCharacter) 0.2))))
    (:then_1
      (|CallParentFunction InBomberCharacter))))

(fn ConstructionScript
  (|CallParentFunction))