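; Timed bomb for a Bomberman-style game that starts blocking pawns once a bomber character stops overlapping it.
; Tick advances a timer that grows the fuse mesh and shifts its dynamic material from yellow toward red, then detonates.
; Explode spawns BP_Explosion at the center and stepwise along each ExplosionTransforms direction up to ExplosionSize, then destroys the bomb.
; WorldStatic sphere overlaps stop a direction by overwriting its vector with a negative-Z sentinel.
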(event Custom|TickBombTimer
  (params (DeltaSeconds :type Float%20%28single-precision%29))
  (Variables|Default|SetBombTimer (+ (Variables|Default|GetBombTimer) DeltaSeconds))
  (Utilities|FlowControl|Sequence
    (:then_0
      (Rendering|Material|SetVectorParameterValue (Variables|Default|GetDynamicFuseMaterial) "Color" (Utilities|Struct|MakeLinearColor 1.0 (- 1.0 (/ (Variables|Default|GetBombTimer) 2.0)) 0.0 1.0) :!class /Script/Engine.MaterialInstanceDynamic))
    (:then_1
      (Transformation|SetRelativeScale3D (Variables|Default|GetFuse) (Math|Vector|MakeVector (/ (Variables|Default|GetBombTimer) (Variables|Default|GetBombFuseTime)) (/ (Variables|Default|GetBombTimer) (Variables|Default|GetBombFuseTime)) (/ (Variables|Default|GetBombTimer) (Variables|Default|GetBombFuseTime)))))
    (:then_2
      (if (> (Variables|Default|GetBombTimer) (Variables|Default|GetBombFuseTime))
        (CallFunction|Explode)))))

(event Custom|Explode
  (Utilities|FlowControl|Sequence
    (:then_0
      (Collision|SetCollisionResponsetoAllChannels (Variables|Default|GetBomb) "ECR_Ignore")
      (Game|SpawnActorfromClass "/Game/Actors/BP_Explosion.BP_Explosion_C" (Transformation|GetActorTransform) "Undefined" 0 0)
      (for _index (range 1 (Variables|Default|GetExplosionSize))
        (for (_array_element _array_index) (Variables|Default|GetExplosionTransforms)
          (bind _returnvalue (Collision|SphereOverlapActors (+ (Transformation|GetActorLocation) (* _array_element _index)) 38.0 (Utilities|Array|MakeArray "ObjectTypeQuery1") 0))
          (if _returnvalue
            (|SetBy-RefVar (Utilities|Array|Get(acopy) (Variables|Default|GetExplosionTransforms) _array_index) "0.000000,0,-1.000000")
            (elif (not (< (.Z (Math|Vector|BreakVector (Utilities|Array|Get(acopy) (Variables|Default|GetExplosionTransforms) _array_index))) 0.0))
              (Game|SpawnActorfromClass "/Game/Actors/BP_Explosion.BP_Explosion_C" (Math|Transform|MakeTransform (+ (Transformation|GetActorLocation) (* _array_element _index)) "0, 0, 0" "1,1,1") "Undefined" 0 0))))))
    (:then_1
      (Actor|DestroyActor))))

(event EventBeginPlay
  (bind _returnvalue (Rendering|Material|CreateDynamicMaterialInstance (Variables|Default|GetFuse) 0 (Rendering|Material|GetMaterial (Variables|Default|GetFuse) 0) :!class /Script/Engine.PrimitiveComponent))
  (Variables|Default|SetDynamicFuseMaterial _returnvalue)
  (Variables|Default|SetDefaultFuseScale (.x (Transformation|GetWorldScale (Variables|Default|GetFuse)))))

(event Collision|EventActorBeginOverlap
  (params (OtherActor :type Actor%20Object%20Reference)))

(event EventTick
  (params (DeltaSeconds :type Float%20%28single-precision%29))
  (CallFunction|TickBombTimer DeltaSeconds))

(event Collision|EventActorEndOverlap
  (params (OtherActor :type Actor%20Object%20Reference))
  (Utilities|Casting|CastToBP_BomberCharacter OtherActor)
  (Collision|SetCollisionResponsetoChannel (Variables|Default|GetBomb) "ECC_Pawn" "ECR_Block"))

(fn ConstructionScript)