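; Game mode for a Bomber game that sets up two local players, each controlling a BP_BomberCharacter.
; BeginPlay switches rendering to unlit through a console command.
; SpawnPlayers spawns characters at the first two PlayerStarts, possessing one with the existing controller and the other with a newly created local player.
; It points the first player's view at the level camera and recolors the second character's sphere with M_Bomber2.
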(event Custom|SpawnPlayers
  (bind _returnvalue (Game|GetPlayerController 0))
  (bind _playerstarts (Variables|Default|GetPlayerStarts))
  (bind _playerstarts_2 (Variables|Default|GetPlayerStarts))
  (bind _output (Utilities|Array|Get(acopy) _playerstarts 1))
  (bind _output_2 (Utilities|Array|Get(acopy) _playerstarts_2))
  (Utilities|FlowControl|Sequence
    (:then_0
      (Utilities|IsValid _output_2
        (:Is%20Valid
          (bind _returnvalue_2 (Game|SpawnActorfromClass "/Game/Characters/BP_BomberCharacter.BP_BomberCharacter_C" (Transformation|GetActorTransform _output_2) "Undefined" 0 0))
          (Utilities|IsValid _returnvalue
            (:Is%20Valid
              (Pawn|Possess _returnvalue _returnvalue_2)
              (Game|Player|SetViewTargetwithBlend _returnvalue (Variables|Default|GetLevelCameraActor) 0.0 "VTBlend_Linear" 0.0 false))))))
    (:then_1
      (Utilities|IsValid _output
        (:Is%20Valid
          (bind _returnvalue_3 (Class|GameplayStatics|CreatePlayer -1))
          (bind _asbp_bomber_player_controller (Utilities|Casting|CastToBP_BomberPlayerController _returnvalue_3))
          (bind _returnvalue_4 (Game|SpawnActorfromClass "/Game/Characters/BP_BomberCharacter.BP_BomberCharacter_C" (Transformation|GetActorTransform _output) "Undefined" 0 0))
          (Pawn|Possess _asbp_bomber_player_controller _returnvalue_4)
          (for _index (range 0 (Rendering|Material|GetNumMaterials (Variables|/Game/Characters/BP_BomberCharacter.BP_BomberCharacter_C|GetSphere _returnvalue_4)))
            (Rendering|Material|SetMaterial (Variables|/Game/Characters/BP_BomberCharacter.BP_BomberCharacter_C|GetSphere _returnvalue_4) _index "/Game/Materials/M_Bomber2.M_Bomber2")))))))

(event EventBeginPlay
  (Development|ExecuteConsoleCommand "viewmode unlit"))

(event EventTick
  (params (DeltaSeconds :type Float%20%28single-precision%29)))

(fn ConstructionScript)