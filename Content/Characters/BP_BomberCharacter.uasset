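; BP_BomberCharacter is a character Blueprint that places bombs on a grid, in the style of Bomberman.
; On the place-bomb event, it uses modulo math to snap the actor's location to a 100-unit cell center at a fixed height.
; A sphere overlap sized by the capsule radius checks that cell for an existing Bomb, and a BP_Bomb spawns only if none is found.
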(event EventBeginPlay)

(event Collision|EventActorBeginOverlap
  (params (OtherActor :type Actor%20Object%20Reference)))

(event EventTick
  (params (DeltaSeconds :type Float%20%28single-precision%29)))

(event EventOnPlaceBombPressed
  (bind _returnvalue (Transformation|GetActorTransform))
  (bind _location (Math|Transform|BreakTransform _returnvalue))
  (bind _location_2 (Math|Transform|BreakTransform _returnvalue))
  (bind _returnvalue_2 (Math|Float|%(Float) (.y _location_2) 1e+02))
  (bind _returnvalue_3 (Math|Float|%(Float) (.x _location_2) 1e+02))
  (bind _returnvalue_4 (- (.x _location) _returnvalue_3))
  (bind _returnvalue_5 (- (.y _location) _returnvalue_2))
  (bind _returnvalue_6 (+ _returnvalue_5 5e+01))
  (bind _returnvalue_7 (+ _returnvalue_4 5e+01))
  (bind _returnvalue_8 (Math|Transform|MakeTransform (Math|Vector|MakeVector _returnvalue_7 _returnvalue_6 5e+01)))
  (bind _returnvalue_9 (Collision|SphereOverlapActors (.Location (Math|Transform|BreakTransform _returnvalue_8)) (Class|CapsuleComponent|GetUnscaledCapsuleRadius (Variables|Default|GetCapsuleComponent)) (Utilities|Array|MakeArray "ObjectTypeQuery1") "/Script/IKABomberman.Bomb"))
  (if (not _returnvalue_9)
    (Game|SpawnActorfromClass "/Game/Actors/BP_Bomb.BP_Bomb_C" _returnvalue_8 "Undefined" 0 0)))

(fn ConstructionScript)